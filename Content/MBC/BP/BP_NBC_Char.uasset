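; BP_NBC_Char is a player character Blueprint that handles basic movement, look and jump through Enhanced Input.
; BeginPlay adds the IA_MBC_MappingDefault mapping context for player controller 0.
; Move input follows control rotation, using yaw for forward and yaw plus roll for right, while Look feeds controller yaw and pitch.
; Jump fires on Started; an actor-right-vector movement call is left unconnected.
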(event `self.ReceiveBeginPlay`
  ; Key Mapping
  (`EnhancedInputSubsystemInterface.AddMappingContext` (pcsubsystem `EnhancedInputLocalPlayerSubsystem` (`GameplayStatics.GetPlayerController` 0)) "/Game/MBC/Inputs/IA_MBC_MappingDefault.IA_MBC_MappingDefault" 0 (struct)))

(event `EnhancedInput|/Game/MBC/Inputs/IA_MBC_Move`
  (params (ActionValue :type "Vector2D Structure") (ElapsedSeconds :type "Float (double-precision)") (TriggeredSeconds :type "Float (double-precision)") (InputAction :type "InputAction Object Reference" :default "/Game/MBC/Inputs/IA_MBC_Move.IA_MBC_Move"))
  (bind (_returnvalue_roll _returnvalue_pitch _returnvalue_yaw) (`KismetMathLibrary.BreakRotator` (`self.GetControlRotation`)))
  (bind (_returnvalue_roll_2 _returnvalue_pitch_2 _returnvalue_yaw_2) (`KismetMathLibrary.BreakRotator` (`self.GetControlRotation`)))
  (:`Triggered`
    (`self.AddMovementInput` (`KismetMathLibrary.GetForwardVector` (`KismetMathLibrary.MakeRotator` 0.0 0.0 _returnvalue_yaw_2)) ActionValue_X)
    (`self.AddMovementInput` (`KismetMathLibrary.GetRightVector` (`KismetMathLibrary.MakeRotator` _returnvalue_roll 0.0 _returnvalue_yaw)) ActionValue_Y)))

(event `EnhancedInput|/Game/MBC/Inputs/IA_MBC_Look`
  (params (ActionValue :type "Vector2D Structure") (ElapsedSeconds :type "Float (double-precision)") (TriggeredSeconds :type "Float (double-precision)") (InputAction :type "InputAction Object Reference" :default "/Game/MBC/Inputs/IA_MBC_Look.IA_MBC_Look"))
  ; 시야
  (:`Triggered`
    (`self.AddControllerYawInput` ActionValue_X)
    (`self.AddControllerPitchInput` ActionValue_Y)))

(event `EnhancedInput|/Game/MBC/Inputs/IA_MBC_Jump`
  (params (ActionValue :type Boolean) (ElapsedSeconds :type "Float (double-precision)") (TriggeredSeconds :type "Float (double-precision)") (InputAction :type "InputAction Object Reference" :default "/Game/MBC/Inputs/IA_MBC_Jump.IA_MBC_Jump"))
  (:`Started`
    (`self.Jump`)))

(fn `UserConstructionScript`)