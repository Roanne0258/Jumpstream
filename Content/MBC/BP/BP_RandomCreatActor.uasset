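; Trigger actor that launches a one-shot randomized attack on one side of the BP_StartFloor when BP_NBC_Char enters its box.
; A random bool picks left or right, then a looping timer spawns BP_Scale actors at random distant points, aimed at that side.
; Each spawn calls a red material blink on that side's platform.
; At the spawn cap the timer clears and a delayed recursive event feeds each actor to a Z-scale timeline.
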(event `self.ReceiveBeginPlay`
  ; 스타트플로어참조
  (bind _outactors (`GameplayStatics.GetAllActorsOfClass` "/Game/MBC/BP/BP_StartFloor.BP_StartFloor_C"))
  (set `self.StartActorReference` (`|GetArrayItem` _outactors)))

(event `self.Box.OnComponentBeginOverlap`
  (params (OverlappedComponent :type "PrimitiveComponent Object Reference") (OtherActor :type "Actor Object Reference") (OtherComp :type "PrimitiveComponent Object Reference") (OtherBodyIndex :type Integer) (bFromSweep :type Boolean) (SweepResult :type "HitResult Structure (by ref)"))
  ; 플레이어가 오버랩이 되는지 확인
  (cast `/Game/MBC/BP/BP_NBC_Char` OtherActor)
  (set `self.random` (`KismetMathLibrary.RandomBool`))
  (`/Engine/EditorBlueprintResources/StandardMacros.DoOnce` false
    (:`Completed`
      (if (not (`self.IsSpawning `))
        (set `self.IsSpawning ` true)
        ; 특정 범위 내 랜덤 위치에 엑터 생성
        (bind _returnvalue (`KismetSystemLibrary.K2_SetTimer` null "SpawnNextActor" 0.04 true))
        (set `self.SpawnTimerHandle ` _returnvalue)))))

(event `StartScaleIncreaseForActor`
  (params (TargetActor :type "Actor Object Reference"))
  (bind (_returnvalue_x _returnvalue_y) (`KismetMathLibrary.BreakVector` (`self.GetActorScale3D` (`self.SpawnActorRef`))))
  ; 스케일 변경
  (bind (_direction _scale) (`Timeline|타임라인`)
    (:`Update`
      (`self.SetActorScale3D` TargetActor (`KismetMathLibrary.MakeVector` _returnvalue_x _returnvalue_y _scale)))))

(event `ProcessNextActor`
  ; 배열 순회해서 엑터 하나마다 스케일 변경 함수 호출
  (if (< (`self.CurrentIndex `) (`self.MaxSpawnCount `))
    (`self.StartScaleIncreaseForActor` (`|GetArrayItem` (`self.SpawnedActorsArray `) (`self.CurrentIndex `)))
    (`KismetSystemLibrary.Delay` 0.02)
    (set `self.CurrentIndex ` (+ (`self.CurrentIndex `) 1))
    (`self.ProcessNextActor`)))

(event `BlinkPlatform_Left`
  (bind _leftparam (`/Game/MBC/BP/BP_StartFloor.GetLeftPlatform` (`self.StartActorReference`)))
  (`PrimitiveComponent.SetMaterial` _leftparam 0 (`self.RedMaterial`))
  (`KismetSystemLibrary.Delay` 0.1)
  (`PrimitiveComponent.SetMaterial` _leftparam 0 (`self.DefaultMaterial`))
  (`KismetSystemLibrary.Delay` 0.1)
  (set `self.BlinkCount ` (+ (`self.BlinkCount `) 1))
  (if (< (`self.BlinkCount `) (`self.MaxBlinkCount`))
    (`self.BlinkPlatform_Left`)))

(event `BlinkPlatform_Right`
  (bind _rightparam (`/Game/MBC/BP/BP_StartFloor.GetRightPlatform` (`self.StartActorReference`)))
  (`PrimitiveComponent.SetMaterial` _rightparam 0 (`self.RedMaterial`))
  (`KismetSystemLibrary.Delay` 0.1)
  (`PrimitiveComponent.SetMaterial` _rightparam 0 (`self.DefaultMaterial`))
  (`KismetSystemLibrary.Delay` 0.1)
  (set `self.BlinkCount ` (+ (`self.BlinkCount `) 1))
  (if (< (`self.BlinkCount `) (`self.MaxBlinkCount`))
    (`self.BlinkPlatform_Right `)))

(fn `SpawnNextActor`
  (locals (NewLocalVar :type "Array of Actor Object Reference") (NewLocalVar_0 :type Integer :default 0))
  (bind (_returnvalue_x _returnvalue_y _returnvalue_z) (`KismetMathLibrary.BreakVector` (`self.K2_GetActorLocation` (`self.StartActorReference`))))
  (bind (_returnvalue_x_2 _returnvalue_y_2 _returnvalue_z_2) (`KismetMathLibrary.BreakVector` (`self.K2_GetActorLocation` (`self.StartActorReference`))))
  (bind (_returnvalue_x_3 _returnvalue_y_3 _returnvalue_z_3) (`KismetMathLibrary.BreakVector` (`self.K2_GetActorLocation` (`self.StartActorReference`))))
  ; 특정 범위내에 스폰 엑터
  (bind _returnvalue (`|SpawnActorFromClass` "/Game/MBC/BP/BP_Scale.BP_Scale_C" (`KismetMathLibrary.MakeTransform` (+ (`KismetMathLibrary.MakeVector` _returnvalue_x _returnvalue_y _returnvalue_z) (`KismetMathLibrary.MakeVector` (`KismetMathLibrary.RandomFloatInRange` -10000.0 10000.0) 15000.0 (`KismetMathLibrary.RandomFloatInRange` 4000.0 10000.0)))) "Undefined" "MultiplyWithRoot" null null))
  ; 생성 엑터들 제어하기 위해서 배열에 넣음
  (`KismetArrayLibrary.Array_Add` (`self.SpawnedActorsArray `) _returnvalue)
  (set `self.SpawnedActorsArray ` (`self.SpawnedActorsArray `))
  ; 50% 확률로 특정 좌표를 향하도록 설정
  (if (`self.random`)
    (`self.BlinkPlatform_Left`)
    (bind _output_get (set `self.SpawnActorRef` _returnvalue))
    (`self.K2_SetActorRotation` _output_get (`KismetMathLibrary.FindLookAtRotation` (`self.K2_GetActorLocation` (`self.SpawnActorRef`)) (`KismetMathLibrary.MakeVector` (+ _returnvalue_x_2 400.0) (+ _returnvalue_y_2 (`KismetMathLibrary.RandomFloatInRange` 100.0 1250.0)) _returnvalue_z_2)) false)
    (else
      (`self.BlinkPlatform_Right `)
      (bind _output_get_2 (set `self.SpawnActorRef` _returnvalue))
      (`self.K2_SetActorRotation` _output_get_2 (`KismetMathLibrary.FindLookAtRotation` (`self.K2_GetActorLocation` (`self.SpawnActorRef`)) (`KismetMathLibrary.MakeVector` (+ _returnvalue_x_3 -400.0) (+ _returnvalue_y_3 (`KismetMathLibrary.RandomFloatInRange` 100.0 1250.0)) _returnvalue_z_3)) false)))
  (set `self.CurrentSpawnCount ` (+ (`self.CurrentSpawnCount `) 1))
  (if (not (< (`self.CurrentSpawnCount `) (`self.MaxSpawnCount `)))
    (`self.ProcessNextActor`)
    (`KismetSystemLibrary.K2_ClearAndInvalidateTimerHandle` (`self.SpawnTimerHandle `))))

(fn `UserConstructionScript`)