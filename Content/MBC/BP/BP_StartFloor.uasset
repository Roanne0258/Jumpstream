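; BP_StartFloor is a floor platform actor with left and right sky bridge pieces that moves at a set velocity.
; On BeginPlay it records its start location, then every Tick it offsets its position by PlatformVelocity scaled by delta time, without sweeping.
; Two getters expose the left and right bridge pieces to other code.
; Tag-based bridge mesh lookup logic remains in the graphs but is disconnected.
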(event `self.ReceiveBeginPlay`
  ; 액터의 기본 위치를 StartLocation 변수에 Set
  (set `self.StartLocation` (`self.K2_GetActorLocation`)))

(event `self.ReceiveTick`
  (params (DeltaSeconds :type "Float (single-precision)"))
  ; 매 프레임마다 속도(Platform Velocity)를 기반으로 플랫폼 위치를 이동시킴.
  (`self.K2_SetActorLocation` (+ (* DeltaSeconds (`self.PlatformVelocity`)) (`self.K2_GetActorLocation`))))

(fn `GetLeftPlatform`
  (returns (LeftParam :type "StaticMeshComponent Object Reference"))
  (return (`self.SM_SkyBridgeLeft`)))

(fn `GetRightPlatform`
  (returns (RightParam :type "StaticMeshComponent Object Reference"))
  (return (`self.SM_SkyBridgeRight`)))

(fn `UserConstructionScript`)