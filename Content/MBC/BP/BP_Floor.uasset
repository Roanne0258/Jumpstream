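; BP_Floor is a floor actor that changes the player character's movement friction while it is inside the floor's Box, apparently to make the surface slippery.
; Tick casts the player pawn to BP_NBC_Char and caches it every frame.
; When that character begins overlapping the Box, its ground friction drops to zero and its braking friction is lowered.
; End overlap sets both to hardcoded higher values rather than restoring saved ones.
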(event `self.ReceiveTick`
  (params (DeltaSeconds :type "Float (single-precision)"))
  (bind _asbp_nbc_char (cast `/Game/MBC/BP/BP_NBC_Char` (`GameplayStatics.GetPlayerPawn` 0)))
  (set `self.As BP NBC Char` _asbp_nbc_char))

(event `self.Box.OnComponentBeginOverlap`
  (params (OverlappedComponent :type "PrimitiveComponent Object Reference") (OtherActor :type "Actor Object Reference") (OtherComp :type "PrimitiveComponent Object Reference") (OtherBodyIndex :type Integer) (bFromSweep :type Boolean) (SweepResult :type "HitResult Structure (by ref)"))
  (bind _charactermovement (`Character.CharacterMovement` (`self.As BP NBC Char`)))
  (if (== OtherActor (`self.As BP NBC Char`))
    (set `CharacterMovementComponent.GroundFriction` 0.0 _charactermovement)
    (set `CharacterMovementComponent.BrakingFriction` 100.0 _charactermovement)))

(event `self.Box.OnComponentEndOverlap`
  (params (OverlappedComponent :type "PrimitiveComponent Object Reference") (OtherActor :type "Actor Object Reference") (OtherComp :type "PrimitiveComponent Object Reference") (OtherBodyIndex :type Integer))
  (bind _charactermovement (`Character.CharacterMovement` (`self.As BP NBC Char`)))
  (if (== OtherActor (`self.As BP NBC Char`))
    (set `CharacterMovementComponent.GroundFriction` 2.0 _charactermovement)
    (set `CharacterMovementComponent.BrakingFriction` 2048.0 _charactermovement)))

(fn `UserConstructionScript`)